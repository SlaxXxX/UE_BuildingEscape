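; Openable door actor that swings open and closed on requests from its OpenDoor event source.
; The construction script stores the initial rotation as the closed pose.
; Open requests play a sound and run a timeline whose curve yaw is combined with that initial rotation to rotate the whole actor.
; Close requests play a separate sound and reverse the same timeline.
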(event OnOpenRequest(OpenDoor)
  (Audio|PlaySoundatLocation "/Game/MyContent/door_open_sound.door_open_sound" (Transformation|GetActorLocation) "0, 0, 0" 1.0 1.0 0.0 0 0 0)
  (bind _timetodoorangle (Timeline|OpenTimeline Play)
    (:Update
      (Transformation|SetActorRotation (Math|Rotator|CombineRotators (Math|Rotator|MakeRotator 0.0 0.0 _timetodoorangle) (Variables|Default|GetinitialRotation))))))

(event OnCloseRequest(OpenDoor)
  (Audio|PlaySoundatLocation "/Game/MyContent/door_close_sound.door_close_sound" (Transformation|GetActorLocation) "0, 0, 0" 1.0 1.0 0.0 0 0 0)
  (bind _timetodoorangle (Timeline|OpenTimeline Reverse)
    (:Update
      (Transformation|SetActorRotation (Math|Rotator|CombineRotators (Math|Rotator|MakeRotator 0.0 0.0 _timetodoorangle) (Variables|Default|GetinitialRotation))))))

(fn ConstructionScript
  (Variables|Default|SetinitialRotation (Transformation|GetActorRotation)))